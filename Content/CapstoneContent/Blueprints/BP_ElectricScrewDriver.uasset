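; BP_ElectricScrewDriver is a grabbable electric screwdriver tool with an animated mesh.
; On BeginPlay it binds to its GrabComponent's grabbed and dropped delegates, passing the held state to ToolGrabbed.
; UseTool loops the screwdriver animation on ElectricToolMesh and StopUsingTool stops it.
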(event `self.ReceiveBeginPlay`
  (bind _grabcomponent (`self.GrabComponent`))
  (add `/Game/VRTemplate/Blueprints/GrabComponent.OnGrabbed` _grabcomponent (delegate `OnGrabbed_Event_0`))
  (add `/Game/VRTemplate/Blueprints/GrabComponent.OnDropped` _grabcomponent (delegate `OnDropped_Event`)))

(event `OnGrabbed_Event_0`
  (`self.ToolGrabbed` true))

(event `OnDropped_Event`
  (`self.ToolGrabbed` false))

(event `self.UseTool`
  (`SkeletalMeshComponent.PlayAnimation` (`self.ElectricToolMesh`) "/Game/CapstoneContent/ElectricScrewDriver_Final2_Anim.ElectricScrewDriver_Final2_Anim" true))

(event `self.StopUsingTool`
  (`SkeletalMeshComponent.Stop` (`self.ElectricToolMesh`)))

(fn `UserConstructionScript`)