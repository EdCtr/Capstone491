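; Electric saw Blueprint for a grabbable tool that animates while in use.
; On BeginPlay it binds to the GrabComponent's grabbed and dropped events, forwarding each to ToolGrabbed as true or false.
; UseTool plays the saw animation on a loop on ElectricToolMesh, and StopUsingTool stops it.
; No cutting or overlap logic is implemented here, and ToolGrabbed is defined outside this graph.
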(event `self.ReceiveBeginPlay`
  (bind _grabcomponent (`self.GrabComponent`))
  (add `/Game/VRTemplate/Blueprints/GrabComponent.OnGrabbed` _grabcomponent (delegate `OnGrabbed_Event_0`))
  (add `/Game/VRTemplate/Blueprints/GrabComponent.OnDropped` _grabcomponent (delegate `OnDropped_Event`)))

(event `OnGrabbed_Event_0`
  (`self.ToolGrabbed` true))

(event `OnDropped_Event`
  (`self.ToolGrabbed` false))

(event `self.UseTool`
  (`SkeletalMeshComponent.PlayAnimation` (`self.ElectricToolMesh`) "/Game/CapstoneContent/Assets/Models/Electric_Saw_Final_Anim.Electric_Saw_Final_Anim" true))

(event `self.StopUsingTool`
  (`SkeletalMeshComponent.Stop` (`self.ElectricToolMesh`)))

(fn `UserConstructionScript`)