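; BP_Leg is a leg actor that deforms as a scalpel cuts it, apparently for a surgery sequence.
; Three collision points respond only to Scapel overlaps, setting the current morph target to zero, half and full weight to show cut progress.
; The final point advances through the MorphNames list to the next morph, and once the list is exhausted it calls OpenMuscleMessage on BP_Muscle.
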(event `self.ReceiveBeginPlay`
  (`self.GetNewMorphTarget`))

(event `self.ReceiveTick`
  (params (DeltaSeconds :type "Float (single-precision)")))

(event `self.CollisionPoint1.OnComponentBeginOverlap`
  (params (OverlappedComponent :type "PrimitiveComponent Object Reference") (OtherActor :type "Actor Object Reference") (OtherComp :type "PrimitiveComponent Object Reference") (OtherBodyIndex :type Integer) (bFromSweep :type Boolean) (SweepResult :type "HitResult Structure (by ref)"))
  (cast `Scapel` OtherActor)
  (`SkeletalMeshComponent.SetMorphTarget` (`self.SkeletalMesh`) (`self.CurrentMorph`) 0.0 true))

(event `self.CollisionPoint2.OnComponentBeginOverlap`
  (params (OverlappedComponent :type "PrimitiveComponent Object Reference") (OtherActor :type "Actor Object Reference") (OtherComp :type "PrimitiveComponent Object Reference") (OtherBodyIndex :type Integer) (bFromSweep :type Boolean) (SweepResult :type "HitResult Structure (by ref)"))
  (cast `Scapel` OtherActor)
  (`SkeletalMeshComponent.SetMorphTarget` (`self.SkeletalMesh`) (`self.CurrentMorph`) 0.5 true))

(event `self.CollisionPoint3.OnComponentBeginOverlap`
  (params (OverlappedComponent :type "PrimitiveComponent Object Reference") (OtherActor :type "Actor Object Reference") (OtherComp :type "PrimitiveComponent Object Reference") (OtherBodyIndex :type Integer) (bFromSweep :type Boolean) (SweepResult :type "HitResult Structure (by ref)"))
  (cast `Scapel` OtherActor)
  (`SkeletalMeshComponent.SetMorphTarget` (`self.SkeletalMesh`) (`self.CurrentMorph`) 1.0 true)
  (bind _result (`/Engine/EditorBlueprintResources/StandardMacros.IncrementInt` (`self.CurrentMorphIndex`))
    (:`  `
      (if (< _result (`KismetArrayLibrary.Array_Length` (`self.MorphNames`)))
        (`self.GetNewMorphTarget`)
        (else
          (bind _returnvalue (`GameplayStatics.GetActorOfClass` "/Game/CapstoneContent/Blueprints/BP_Muscle.BP_Muscle_C"))
          (message `/Game/CapstoneContent/Blueprints/BPI_Muscle.OpenMuscle` _returnvalue))))))

(fn `GetNewMorphTarget`
  (set `self.CurrentMorph` (`|GetArrayItem` (`self.MorphNames`) (`self.CurrentMorphIndex`))))

(fn `UserConstructionScript`)