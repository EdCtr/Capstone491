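; BP_Muscle is the hip surgery site actor, holding muscle, fascia and femur meshes and moving the surgery forward through BP_Game phases.
; OpenMuscle and CloseMuscle use timelines to drive morph targets and slide assistant retractor hands, then set the exposure or congrats phase on finish.
; Overlap volumes detect saw, forceps, screwdriver and cup items to trigger later phases, with flags guarding most steps and the removed bone snapping to the forceps.
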(event `/Game/CapstoneContent/Blueprints/BPI_Muscle.CloseMuscle`
  (bind _fascia_lata (`self.Fascia_lata`))
  (bind _returnvalue (`GameplayStatics.GetActorOfClass` "/Game/CapstoneContent/Blueprints/BP_Leg.BP_Leg_C"))
  (set `self.BP_LegRef` _returnvalue)
  (`SceneComponent.SetVisibility` (`self.Assistant_Holding_Upper_Retractor`) true false)
  (`SceneComponent.SetVisibility` (`self.Assistant_Holding_Lower_Retractor`) true false)
  (bind (_direction _muscleanimation) (`Timeline|Timeline_1`)
    (:`Update`
      (bind _returnvalue_2 (`KismetMathLibrary.Lerp` 0.0 1.0 _muscleanimation))
      (`SkeletalMeshComponent.SetMorphTarget` (`self.Gluteus_Medius_Muscle`) "Gluteus_medius_Pull" _returnvalue_2 true)
      (`SkeletalMeshComponent.SetMorphTarget` _fascia_lata "Fascia_End" _returnvalue_2 true)
      (`SkeletalMeshComponent.SetMorphTarget` (`self.Gluteus_Minimus_Muscle`) "Gluteus_minimus_Pull" _returnvalue_2 true)
      (`SkeletalMeshComponent.SetMorphTarget` _fascia_lata "Fascia_Start" _returnvalue_2 true)
      (`SkeletalMeshComponent.SetMorphTarget` (`self.Rectus_Femoris_Muscle`) "Rectus_Pull" _returnvalue_2 true)
      (`SkeletalMeshComponent.SetMorphTarget` (`self.Tensor_Fasciae_Latae`) "Tensor_Pull" _returnvalue_2 true)
      (`SkeletalMeshComponent.SetMorphTarget` (`self.Femur`) "Key 1" _returnvalue_2 true)
      (`SkeletalMeshComponent.SetMorphTarget` (`/Game/CapstoneContent/Blueprints/BP_Leg.SkeletalMesh` (`self.BP_LegRef`)) "Skin_Pull" 0.0 true)
      (bind _returnvalue_3 (`KismetMathLibrary.Lerp` 0.0 1.0 _returnvalue_2))
      (`SceneComponent.K2_SetWorldLocation` (`self.Assistant_Holding_Upper_Retractor`) (`KismetMathLibrary.VLerp` (`SceneComponent.K2_GetComponentLocation` (`self.Assistant_Holding_Upper_Retractor`)) (`SceneComponent.K2_GetComponentLocation` (`self.HandStartPosUpper`)) _returnvalue_3) false false)
      (`SceneComponent.K2_SetWorldLocation` (`self.Assistant_Holding_Lower_Retractor`) (`KismetMathLibrary.VLerp` (`SceneComponent.K2_GetComponentLocation` (`self.Assistant_Holding_Lower_Retractor`)) (`SceneComponent.K2_GetComponentLocation` (`self.HandStartPosLower`)) _returnvalue_3) false false))
    (:`Finished`
      (`SceneComponent.SetVisibility` (`self.Assistant_Holding_Upper_Retractor`) false false)
      (`SceneComponent.SetVisibility` (`self.Assistant_Holding_Lower_Retractor`) false false)
      (bind _returnvalue_4 (`GameplayStatics.GetActorOfClass` "/Game/CapstoneContent/Blueprints/BP_Game.BP_Game_C"))
      (`Game.SetSurgeryPhase` _returnvalue_4 "CONGRATS")
      (`Game.ExecuteGamePhase` _returnvalue_4))))

(event `self.ReceiveBeginPlay`
  (`SceneComponent.K2_SetWorldLocation` (`self.HandStartPosUpper`) (`SceneComponent.K2_GetComponentLocation` (`self.Assistant_Holding_Upper_Retractor`)) false false)
  (`SceneComponent.K2_SetWorldLocation` (`self.HandStartPosLower`) (`SceneComponent.K2_GetComponentLocation` (`self.Assistant_Holding_Lower_Retractor`)) false false))

(event `/Game/CapstoneContent/Blueprints/BPI_Muscle.OpenMuscle`
  (bind _fascia_lata (`self.Fascia_lata`))
  (`SceneComponent.SetVisibility` (`self.Assistant_Holding_Upper_Retractor`) true false)
  (`SceneComponent.SetVisibility` (`self.Assistant_Holding_Lower_Retractor`) true false)
  (bind (_direction _muscleanimation) (`Timeline|Timeline`)
    (:`Update`
      (bind _returnvalue (`KismetMathLibrary.Lerp` 0.0 1.0 _muscleanimation))
      (`SkeletalMeshComponent.SetMorphTarget` (`self.Gluteus_Medius_Muscle`) "Gluteus_medius_Pull" _returnvalue true)
      (`SkeletalMeshComponent.SetMorphTarget` _fascia_lata "Fascia_End" _returnvalue true)
      (`SkeletalMeshComponent.SetMorphTarget` (`self.Gluteus_Minimus_Muscle`) "Gluteus_minimus_Pull" _returnvalue true)
      (`SkeletalMeshComponent.SetMorphTarget` _fascia_lata "Fascia_Start" _returnvalue true)
      (`SkeletalMeshComponent.SetMorphTarget` (`self.Rectus_Femoris_Muscle`) "Rectus_Pull" _returnvalue true)
      (`SkeletalMeshComponent.SetMorphTarget` (`self.Tensor_Fasciae_Latae`) "Tensor_Pull" _returnvalue true)
      (`SceneComponent.K2_SetWorldLocation` (`self.Assistant_Holding_Upper_Retractor`) (`KismetMathLibrary.VLerp` (`SceneComponent.K2_GetComponentLocation` (`self.Assistant_Holding_Upper_Retractor`)) (`SceneComponent.K2_GetComponentLocation` (`self.HandEndPosUpper`)) _returnvalue) false false)
      (`SceneComponent.K2_SetWorldLocation` (`self.Assistant_Holding_Lower_Retractor`) (`KismetMathLibrary.VLerp` (`SceneComponent.K2_GetComponentLocation` (`self.Assistant_Holding_Lower_Retractor`)) (`SceneComponent.K2_GetComponentLocation` (`self.HandEndPosLower`)) _returnvalue) false false))
    (:`Finished`
      (`SceneComponent.SetVisibility` (`self.Assistant_Holding_Upper_Retractor`) false false)
      (`SceneComponent.SetVisibility` (`self.Assistant_Holding_Lower_Retractor`) false false)
      (bind _returnvalue_2 (`GameplayStatics.GetActorOfClass` "/Game/CapstoneContent/Blueprints/BP_Game.BP_Game_C"))
      (`Game.SetSurgeryPhase` _returnvalue_2 "EXPOSURE")
      (`Game.ExecuteGamePhase` _returnvalue_2))))

(event `self.FemoralSawCollision.OnComponentBeginOverlap`
  (params (OverlappedComponent :type "PrimitiveComponent Object Reference") (OtherActor :type "Actor Object Reference") (OtherComp :type "PrimitiveComponent Object Reference") (OtherBodyIndex :type Integer) (bFromSweep :type Boolean) (SweepResult :type "HitResult Structure (by ref)"))
  (cast `/Game/CapstoneContent/Blueprints/BP_ElectricSaw` OtherActor)
  (bind _returnvalue (`GameplayStatics.GetActorOfClass` "/Game/CapstoneContent/Blueprints/BP_Game.BP_Game_C"))
  (`Game.SetSurgeryPhase` _returnvalue "REMOVAL")
  (`Game.ExecuteGamePhase` _returnvalue))

(event `self.Femur_Forcep_Grab_Collision.OnComponentBeginOverlap`
  (params (OverlappedComponent :type "PrimitiveComponent Object Reference") (OtherActor :type "Actor Object Reference") (OtherComp :type "PrimitiveComponent Object Reference") (OtherBodyIndex :type Integer) (bFromSweep :type Boolean) (SweepResult :type "HitResult Structure (by ref)"))
  (`|ExecutionSequence`
    (:`then_0`
      (bind _asbp_forceps (cast `/Game/CapstoneContent/Blueprints/BP_Forceps` OtherActor))
      (`SceneComponent.K2_AttachToComponent` (`self.Femur_Removal_Bone`) (`/Game/CapstoneContent/Blueprints/BP_Forceps.FemoralHeadLocation` _asbp_forceps) "None" "SnapToTarget" "SnapToTarget" "SnapToTarget" true))
    (:`then_1`
      (if (and (== (`KismetSystemLibrary.GetDisplayName` OtherActor) "Rolling_Table__1_") (not (`self.bFemurBoneRemoved`)))
        (`KismetSystemLibrary.PrintString` "Yes It be" true true (struct :`G` 0.66 :`B` 1.0 :`A` 1.0) 200.0)
        (set `self.bFemurBoneRemoved` true)
        (bind _returnvalue (`GameplayStatics.GetActorOfClass` "/Game/CapstoneContent/Blueprints/BP_Game.BP_Game_C"))
        (`Game.SetSurgeryPhase` _returnvalue "REAMING")
        (`Game.ExecuteGamePhase` _returnvalue)
        (bind (_direction _muscleanimation) (`Timeline|Timeline_0`)
          (:`Update`
            (`SkeletalMeshComponent.SetMorphTarget` (`self.Femur`) "Key 1" _muscleanimation true)))))))

(event `self.ReamingCollision.OnComponentBeginOverlap`
  (params (OverlappedComponent :type "PrimitiveComponent Object Reference") (OtherActor :type "Actor Object Reference") (OtherComp :type "PrimitiveComponent Object Reference") (OtherBodyIndex :type Integer) (bFromSweep :type Boolean) (SweepResult :type "HitResult Structure (by ref)"))
  (`|ExecutionSequence`
    (:`then_0`
      (if (not (`self.bReamingCompleted`))
        (cast `ElectricScrewDriver` OtherActor)
        (set `self.bReamingCompleted` true)
        (bind _returnvalue (`GameplayStatics.GetActorOfClass` "/Game/CapstoneContent/Blueprints/BP_Game.BP_Game_C"))
        (`Game.SetSurgeryPhase` _returnvalue "CUPPA")
        (`Game.ExecuteGamePhase` _returnvalue)))
    (:`then_1`
      (cast `/Game/CapstoneContent/Blueprints/BP_CuppaItem` OtherActor)
      (if (`self.bCupPlaced`)
        (if (not (`self.bLinerPlaced`))
          (set `self.bLinerPlaced` true)
          (bind _returnvalue_2 (`GameplayStatics.GetActorOfClass` "/Game/CapstoneContent/Blueprints/BP_Game.BP_Game_C"))
          (`Game.SetSurgeryPhase` _returnvalue_2 "BROACHING")
          (`Game.ExecuteGamePhase` _returnvalue_2))
        (else
          (set `self.bCupPlaced` true))))))

(fn `UserConstructionScript`)